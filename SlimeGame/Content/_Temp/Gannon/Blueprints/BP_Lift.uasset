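; BP_Lift is a moving lift platform that responds to the side-scroller character standing in its trigger.
; Entering LiftTrigger plays a timeline, which lerps the LiftMesh relative location from LiftStartPosition to LiftEndPosition without sweeping.
; Leaving the trigger reverses the timeline, sending the lift back toward its start from wherever it is.
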(event OnComponentBeginOverlap(LiftTrigger)
  (params (OverlappedComponent :type Primitive%20Component%20Object%20Reference) (OtherActor :type Actor%20Object%20Reference) (OtherComp :type Primitive%20Component%20Object%20Reference) (OtherBodyIndex :type Integer) (bFromSweep :type Boolean) (SweepResult :type Hit%20Result%20Structure%20%28by%20ref%29))
  (Utilities|Casting|CastToSideScrollerCharacter OtherActor)
  (bind _alpha (Timeline|Timeline_0 Play)
    (:Update
      (Transformation|SetRelativeLocation (Variables|Default|GetLiftMesh) (Math|Vector|Lerp(Vector) (Variables|/Script/Engine.SceneComponent|GetRelativeLocation (Variables|Default|GetLiftStartPosition)) (Variables|/Script/Engine.SceneComponent|GetRelativeLocation (Variables|Default|GetLiftEndPosition)) _alpha) false false))))

(event OnComponentEndOverlap(LiftTrigger)
  (params (OverlappedComponent :type Primitive%20Component%20Object%20Reference) (OtherActor :type Actor%20Object%20Reference) (OtherComp :type Primitive%20Component%20Object%20Reference) (OtherBodyIndex :type Integer))
  (Utilities|Casting|CastToSideScrollerCharacter OtherActor)
  (bind _alpha (Timeline|Timeline_0 Reverse)
    (:Update
      (Transformation|SetRelativeLocation (Variables|Default|GetLiftMesh) (Math|Vector|Lerp(Vector) (Variables|/Script/Engine.SceneComponent|GetRelativeLocation (Variables|Default|GetLiftStartPosition)) (Variables|/Script/Engine.SceneComponent|GetRelativeLocation (Variables|Default|GetLiftEndPosition)) _alpha) false false))))

(fn ConstructionScript)