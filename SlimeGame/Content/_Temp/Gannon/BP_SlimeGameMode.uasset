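; BP_SlimeGameMode is a game mode that creates the UI and respawns the side-scroller player character when it is destroyed.
; BeginPlay and Respawn share one path that adds a new BP_UI widget to the viewport and binds to the character's OnDestroyed.
; On destruction, it waits briefly, spawns and possesses a new SideScrollerCharacter at SpawnTransform, then calls Respawn, adding another widget without removing the previous one.
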(event Custom|OnDestroyed_Event_0
  (params (DestroyedActor :type Actor%20Object%20Reference))
  (Utilities|FlowControl|Delay 1.0)
  (bind _returnvalue (Game|SpawnActorfromClass "/Game/SideScrollerBP/Blueprints/SideScrollerCharacter.SideScrollerCharacter_C" (Variables|Default|GetSpawnTransform) "Undefined" 0 0))
  (Pawn|Possess (Game|GetPlayerController 0) _returnvalue)
  (CallFunction|Respawn))

(event Custom|Respawn
  (bind _returnvalue (UserInterface|CreateWidget "/Game/_Temp/Gannon/UI/BP_UI.BP_UI_C"))
  (UserInterface|Viewport|AddtoViewport _returnvalue 0)
  (bind _asside_scroller_character (Utilities|Casting|CastToSideScrollerCharacter (Game|GetPlayerCharacter 0)))
  (Game|AssignOnDestroyed _asside_scroller_character (delegate Custom|OnDestroyed_Event_0)))

(event EventBeginPlay
  (bind _returnvalue (UserInterface|CreateWidget "/Game/_Temp/Gannon/UI/BP_UI.BP_UI_C"))
  (UserInterface|Viewport|AddtoViewport _returnvalue 0)
  (bind _asside_scroller_character (Utilities|Casting|CastToSideScrollerCharacter (Game|GetPlayerCharacter 0)))
  (Game|AssignOnDestroyed _asside_scroller_character (delegate Custom|OnDestroyed_Event_0)))

(fn ConstructionScript)