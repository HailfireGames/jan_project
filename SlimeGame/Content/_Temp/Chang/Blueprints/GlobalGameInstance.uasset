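; Global game instance Blueprint that classifies a Health value into Light, Normal or Heavy tiers.
; Three functions, IsLight, IsNormal and IsHeavy, compare the input against the "Light" and "Heavy" entries of the HealthThresholds map.
; Light and Heavy include their threshold values, while Normal covers only values strictly between the two.
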(fn IsHeavy
  (params (health :type Integer))
  (return (>= health (.Value (Utilities|Map|Find (Variables|Default|Get_HealthThresholds) "Heavy")))))

(fn IsLight
  (params (health :type Integer))
  (return (<= health (.Value (Utilities|Map|Find (Variables|Default|Get_HealthThresholds) "Light")))))

(fn IsNormal
  (params (health :type Integer))
  (bind __healththresholds (Variables|Default|Get_HealthThresholds))
  (return (and (> health (.Value (Utilities|Map|Find __healththresholds "Light"))) (< health (.Value (Utilities|Map|Find __healththresholds "Heavy"))))))