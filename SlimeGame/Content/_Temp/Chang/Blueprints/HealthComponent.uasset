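; Actor component that tracks a Health value and translates it into a size category.
; DecrementHealth and IncrementHealth subtract from or add to Health directly, without clamping.
; GetSize scans the HealthThresholds map values in stored order, stops at the first one Health does not exceed, and returns the key at that index, so results depend on entry order.
; BeginPlay and Tick are unused.
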(event EventBeginPlay)

(event EventTick
  (params (DeltaSeconds :type Float%20%28single-precision%29)))

(fn DecrementHealth
  (params (DecrementVal :type Integer))
  (Variables|Default|Set_Health (- (Variables|Default|Get_Health) DecrementVal)))

(fn IncrementHealth
  (params (IncrementVal :type Integer))
  (Variables|Default|Set_Health (+ (Variables|Default|Get_Health) IncrementVal)))

(fn GetSize
  (bind _healththresholds (Variables|Default|GetHealthThresholds))
  (bind _values (Utilities|Map|Values _healththresholds))
  (bind _index (Utilities|FlowControl|ForLoopwithBreak 0 (Utilities|Array|Length _values) :!label _label)
    (:LoopBody
      (if (<= (Variables|Default|Get_Health) (Utilities|Array|Get(acopy) _values _index))
        (goto _label Break)))
    (:Completed
      (bind _keys (Utilities|Map|Keys _healththresholds))
      (return (Utilities|Array|Get(acopy) _keys _index)))))